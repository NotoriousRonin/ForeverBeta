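; Player character for a 2D side-scroller, handling movement, jumping, sliding, damage, death and bug-collecting score.
; A CharState value picks the sprite flipbook each Tick, which also forces movement while sliding or sets facing via control rotation.
; Damage knocks the character back; landing restores control or triggers death music and a replay widget.
; BeginPlay creates the HUD and loads the high score; the websocket remote-control handler exists, but its connection code never runs.
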(event `OnReceiveData_Event_0`
  (params (data :type String))
  (bind _issliding (`self.isSliding`))
  ;[1 0.8571 0] Initialize
  ;;[1 1 1] Websocket
  ;;;[1 1 1] Auslagern der Steuerung
  (switch `string` data
    (:`Jump`
      (`self.Jump`)
      (set `self.char_state` "NewEnumerator2"))
    (:`Left`
      (if (not _issliding)
        (set `self.bisMovingRight` false)
        (`self.AddMovementInput` (1.0 0.0 0.0) :!label _label)))
    (:`Right`
      (if (not _issliding)
        (set `self.bisMovingRight` true)
        (goto _label)))))

(event `self.ReceiveBeginPlay`
  ;[1 0.8571 0] Initialize
  (`|ExecutionSequence`
    (:`then_0`
      (`AudioComponent.Play` (`self.PlayBackgroundMusic`) 0.0))
    (:`then_1`
      (`self.LadeHighScore`)
      (`ActorComponent.SetIsReplicated` (`self.Sprite`) true))
    (:`then_2`
      (bind _returnvalue (`|CreateWidget` "/Game/Blueprints/Widget_HUD.Widget_HUD_C" (`GameplayStatics.GetPlayerController` 0)))
      (bind _output_get (set `self.hud_ingame` _returnvalue))
      (`UserWidget.AddToViewport` _output_get 0))))

(event `UpdateAnimation`
  ;[0.07934 0 0.8854] Animation Updater
  (switch `/Game/Blueprints/Character_States` (`self.char_state`)
    (:`NewEnumerator0`
      (`PaperFlipbookComponent.SetFlipbook` (`self.Sprite`) (select `bool` (> (`KismetMathLibrary.VSize` (`self.GetVelocity`)) 0.0) :`false` "/Game/Sprites/Charakter/A_Stance.A_Stance" :`true` "/Game/Sprites/Charakter/A_Run.A_Run" :!type "PaperFlipbook Object Reference")))
    (:`NewEnumerator2`
      (`PaperFlipbookComponent.SetFlipbook` (`self.Sprite`) "/Game/Sprites/Charakter/A_Jump.A_Jump"))
    (:`NewEnumerator4`
      (`PaperFlipbookComponent.SetFlipbook` (`self.Sprite`) "/Game/Sprites/Charakter/A_Hit.A_Hit"))
    (:`NewEnumerator5`
      (`PaperFlipbookComponent.SetFlipbook` (`self.Sprite`) "/Game/Sprites/Charakter/A_Dead.A_Dead"))
    (:`NewEnumerator6`
      (`PaperFlipbookComponent.SetFlipbook` (`self.Sprite`) "/Game/Sprites/Charakter/A_Sitting.A_Sitting"))
    (:`NewEnumerator7`
      (`PaperFlipbookComponent.SetFlipbook` (`self.Sprite`) "/Game/Sprites/Charakter/A_Slide.A_Slide"))))

(event `Play Hit Sound`
  ;[1 0.02348 0] Sound Events
  ;;[1 0.02348 0] Hit Sound
  (switch `int` (`KismetMathLibrary.RandomIntegerInRange` 0 1)
    (:`0`
      (`GameplayStatics.SpawnSoundAtLocation` "/Game/Sound/SoundCues/Hit/Jab-SoundBible_com-1806727891_Cue.Jab-SoundBible_com-1806727891_Cue"))
    (:`1`
      (`GameplayStatics.SpawnSoundAtLocation` "/Game/Sound/SoundCues/Hit/Upper_Cut-SoundBible_com-1272257235_Cue.Upper_Cut-SoundBible_com-1272257235_Cue"))))

(event `InputAxis|MoveRight`
  (params (AxisValue :type "Float (single-precision)"))
  ;[0.07934 0 0.8854] Character Movement
  (if (not (`|EnumEquality` (`self.char_state`) "NewEnumerator7"))
    (`/Engine/EditorBlueprintResources/StandardMacros.CompareFloat` AxisValue
      (:`>`
        (set `self.bisMovingRight` true))
      (:`<`
        (set `self.bisMovingRight` false)))
    (`self.AddMovementInput` (1.0 0.0 0.0) AxisValue)))

(event `Play Dead Sound`
  ;[1 0.02348 0] Sound Events
  ;;[1 0.02348 0] Dead Sound
  (switch `int` (`KismetMathLibrary.RandomIntegerInRange` 0 3)
    (:`0`
      (`GameplayStatics.SpawnSoundAtLocation` "/Game/Sound/SoundCues/Dead/Death_Is_Just_Another_Path_Cue.Death_Is_Just_Another_Path_Cue"))
    (:`1`
      (`GameplayStatics.SpawnSoundAtLocation` "/Game/Sound/SoundCues/Dead/Naruto_Shippuden_OST_Original_Soundtrack_14_-_Nightfall_Cue.Naruto_Shippuden_OST_Original_Soundtrack_14_-_Nightfall_Cue"))
    (:`2`
      (`GameplayStatics.SpawnSoundAtLocation` "/Game/Sound/SoundCues/Dead/Naruto_-_Shippuuden_Cue.Naruto_-_Shippuuden_Cue"))
    (:`3`
      (`GameplayStatics.SpawnSoundAtLocation` "/Game/Sound/SoundCues/Dead/Bleach_-_OST_Cue.Bleach_-_OST_Cue"))))

(event `DamageInput`
  (params (`Damage In` :type "Float (double-precision)"))
  ;[0 1 0.05951] Damage Input
  (`self.Play Hit Sound`)
  (set `self.isHit` true)
  (`self.DisableInput` (`GameplayStatics.GetPlayerController` 0))
  (set `self.health_current` (- (`self.health_current`) `Damage In`))
  (`|ExecutionSequence`
    (:`then_0`
      (set `self.char_state` "NewEnumerator4")
      (`MovementComponent.StopMovementImmediately` (`self.CharacterMovement`))
      (`CharacterMovementComponent.AddForce` (`self.CharacterMovement`) (-500000.0 0.0 4500000.0)))))

(event `self.OnLanded`
  (params (Hit :type "HitResult Structure (by ref)"))
  ;[0.07934 0 0.8854] Landing
  (if (`self.isHit`)
    ;;[1 1 1] ifHit
    (set `self.char_state` "NewEnumerator6")
    (`self.UpdateAnimation`)
    (`KismetSystemLibrary.Delay` 0.3)
    (set `self.isHit` false)
    (if (<= (`self.health_current`) 0.0)
      (set `self.char_state` "NewEnumerator5")
      (`self.DisableInput` (`GameplayStatics.GetPlayerController` 0))
      (`self.SetActorEnableCollision` false)
      (`AudioComponent.Stop` (`self.PlayBackgroundMusic`))
      (`self.Play Dead Sound`)
      (`KismetSystemLibrary.Delay` 3.0)
      (`self.Charackter tot`)
      (else
        (set `self.char_state` "NewEnumerator0")
        (`self.UpdateAnimation`)
        (`self.EnableInput` (`GameplayStatics.GetPlayerController` 0))))
    (elif (not (`self.isSliding`))
      (`self.Play Landing Sound`)
      (set `self.char_state` "NewEnumerator0")
      (`self.UpdateAnimation`))))

(event `Play Item Sound`
  ;[1 0.02348 0] Sound Events
  ;;[1 0.02348 0] Item Sound
  (`GameplayStatics.SpawnSoundAtLocation` "/Game/Sound/SoundCues/Item/item_Cue.item_Cue"))

(event `InputAction|Jump`
  (params (Key :type "Key Structure"))
  ;[0.07934 0 0.8854] Jumping
  (:`Pressed`
    (`self.Jump`)
    (set `self.char_state` "NewEnumerator2")
    (`self.Play Jump Sound`))
  (:`Released`
    (`self.StopJumping`)))

(event `self.ReceiveTick`
  (params (DeltaSeconds :type "Float (single-precision)"))
  (bind _returnvalue (`GameplayStatics.GetPlayerController` 0))
  (bind _returnvalue_x (`KismetMathLibrary.BreakVector` (`self.GetVelocity`)))
  ;[0.6076 0 0.8854] Event Tick
  (`self.UpdateAnimation`)
  (if (`self.isSliding`)
    (`self.AddMovementInput` (1.0 0.0 0.0))
    (else
      ;;[1 1 1] Direction Change
      (`/Engine/EditorBlueprintResources/StandardMacros.CompareFloat` _returnvalue_x
        (:`>`
          (`Controller.SetControlRotation` _returnvalue (`KismetMathLibrary.MakeRotator` 0.0) :!label _label_2))
        (:`==`
          (if (`self.bisMovingRight`)
            (goto _label_2)
            (else
              (`Controller.SetControlRotation` _returnvalue (`KismetMathLibrary.MakeRotator` 0.0 0.0 180.0) :!label _label_3))))
        (:`<`
          (goto _label_3))))))

(event `Play Landing Sound`
  ;[1 0.02348 0] Sound Events
  ;;[1 0.02348 0] Landing Sound
  (`GameplayStatics.SpawnSoundAtLocation` "/Game/Sound/SoundCues/Walk/stepstone_1_Cue.stepstone_1_Cue"))

(event `Play Jump Sound`
  ;[1 0.02348 0] Sound Events
  ;;[1 0.02348 0] Jump Sound
  (if (< (`self.JumpCurrentCount`) 1)
    (`GameplayStatics.SpawnSoundAtLocation` "/Game/Sound/SoundCues/Jump/Mario-jump-sound_Cue.Mario-jump-sound_Cue")))

(event `Charackter tot`
  ;[1 1 1] ReplayGame
  (bind _returnvalue (`|CreateWidget` "/Game/Hauptmenü/ReplayOrExit_Widget.ReplayOrExit_Widget_C"))
  (`UserWidget.AddToViewport` _returnvalue 0)
  (set `PlayerController.bShowMouseCursor` true (`GameplayStatics.GetPlayerController` 0)))

(event `LadeHighScore`
  ;[1 1 1] Lädt Highscore/setHighscore
  (bind _returnvalue (`GameplayStatics.DoesSaveGameExist` "Slot1"))
  (if _returnvalue
    (bind _returnvalue_2 (`GameplayStatics.LoadGameFromSlot` "Slot1"))
    (bind _output_get (set `self.HighScoreSpeicher` _returnvalue_2))
    (bind _asspeicher_klasse (cast `/Game/Blueprints/SpielSpeichern/SpeicherKlasse` _output_get))
    (set `self.highscore` (`/Game/Blueprints/SpielSpeichern/SpeicherKlasse.1_Highscore` _asspeicher_klasse))))

(fn `collectBugs`
  (params (NewParam :type Integer))
  ;[1 1 1] Zählt den Highscore hoch sobald dieser niedriger ist als Score
  (set `self.score` (+ NewParam (`self.score`)))
  (if (< (`self.highscore`) (`self.score`))
    (set `self.isHighscoreErreicht` true)
    (set `self.highscore` (`self.score`))))

(fn `UserConstructionScript`)