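; BP_Enemy is a 2D flipbook enemy that patrols between two points and damages BP_Character on contact.
; The construction script builds relative InterpToMovement control points from PointA and PointB, and a FlipFlop turns the sprite on each reversal.
; Box overlap passes DamageValue to the character's DamageInput, then switches off the enemy's collision for two seconds if the character is in a specific state.
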(event `self.InterpToMovement.OnInterpToReverse`
  (params (ImpactResult :type "HitResult Structure (by ref)") (Time :type "Float (single-precision)"))
  (bind _paperflipbook (`self.PaperFlipbook`))
  (`/Engine/EditorBlueprintResources/StandardMacros.FlipFlop`
    (:`A`
      (`SceneComponent.K2_SetWorldRotation` _paperflipbook (struct) false false))
    (:`B`
      (`SceneComponent.K2_SetWorldRotation` _paperflipbook (struct :`Yaw` 180.0) false false))))

(event `self.Box.OnComponentBeginOverlap`
  (params (OverlappedComponent :type "PrimitiveComponent Object Reference") (OtherActor :type "Actor Object Reference") (OtherComp :type "PrimitiveComponent Object Reference") (OtherBodyIndex :type Integer) (bFromSweep :type Boolean) (SweepResult :type "HitResult Structure (by ref)"))
  (bind _asbp_character (cast `/Game/Blueprints/BP_Character` OtherActor))
  (`/Game/Blueprints/BP_Character.DamageInput` _asbp_character (`self.damage_value`))
  (if (`|EnumEquality` (`/Game/Blueprints/BP_Character.char_state` _asbp_character) "NewEnumerator4")
    (`self.SetActorEnableCollision` false)
    (`KismetSystemLibrary.Delay` 2.0)
    (`self.SetActorEnableCollision` true)))

(fn `UserConstructionScript`
  (set `InterpToMovementComponent.ControlPoints` (`|MakeArray` (make `InterpControlPoint` (`self.PointA`)) (make `InterpControlPoint` (`self.PointB`))) (`self.InterpToMovement`)))