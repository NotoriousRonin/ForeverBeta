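; BP_Levelloader is a one-shot trigger that streams in a random next level segment when BP_Character overlaps its box.
; It rerolls the character's NextLevel until it differs from CurrentLevel, then loads the matching numbered "Level_" map as a level instance.
; Each instance is placed further along X at a fixed spacing scaled by the character's CountLevel.
; It then updates the character's CurrentLevel and CountLevel and destroys itself.
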(event `self.Box.OnComponentBeginOverlap`
  (params (OverlappedComponent :type "PrimitiveComponent Object Reference") (OtherActor :type "Actor Object Reference") (OtherComp :type "PrimitiveComponent Object Reference") (OtherBodyIndex :type Integer) (bFromSweep :type Boolean) (SweepResult :type "HitResult Structure (by ref)"))
  ;[1 1 1] Level Loader
  (bind _asbp_character (cast `/Game/Blueprints/BP_Character` OtherActor))
  (while (== (`/Game/Blueprints/BP_Character.nextLevel` _asbp_character) (`/Game/Blueprints/BP_Character.currentLevel` _asbp_character))
    (set `/Game/Blueprints/BP_Character.nextLevel` (`KismetMathLibrary.RandomIntegerInRange` 1 6) _asbp_character))
  (`LevelStreamingKismet.LoadLevelInstance` (`KismetStringLibrary.BuildString_Int` "Level_" "" (`/Game/Blueprints/BP_Character.nextLevel` _asbp_character)) (`KismetMathLibrary.MakeVector` (* 547.0 (`KismetMathLibrary.Conv_IntToDouble` (+ (`/Game/Blueprints/BP_Character.countLevel` _asbp_character) 1)))))
  (set `/Game/Blueprints/BP_Character.currentLevel` (`/Game/Blueprints/BP_Character.nextLevel` _asbp_character) _asbp_character)
  (set `/Game/Blueprints/BP_Character.countLevel` (+ (`/Game/Blueprints/BP_Character.countLevel` _asbp_character) 1) _asbp_character)
  (`self.K2_DestroyActor`))

(fn `UserConstructionScript`)