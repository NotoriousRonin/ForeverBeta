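; Monitor Blueprint that toggles a single monitor on and off when its BoxB1 component registers a hit.
; A boolean flips on each hit to switch visibility between the Aus (off) component and the Loading component.
; Switching on plays Loading from the start without looping, and both states print a debug string.
; The hit event has no filter or debounce, so every hit toggles the state.
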(event `self.BoxB1.OnComponentHit`
  (params (HitComponent :type "PrimitiveComponent Object Reference") (OtherActor :type "Actor Object Reference") (OtherComp :type "PrimitiveComponent Object Reference") (NormalImpulse :type "Vector Structure") (Hit :type "HitResult Structure (by ref)"))
  (bind _aus (`self.Aus`))
  (bind _loading (`self.Loading`))
  (if (`self.isTouched_Monitor1`)
    (set `self.isTouched_Monitor1` false)
    (`KismetSystemLibrary.PrintString` "AUS")
    (`SceneComponent.SetVisibility` _aus true false)
    (`SceneComponent.SetVisibility` _loading false false)
    (else
      (set `self.isTouched_Monitor1` true)
      (`KismetSystemLibrary.PrintString` "AN")
      (`SceneComponent.SetVisibility` _aus false false)
      (`SceneComponent.SetVisibility` _loading true false)
      (`PaperFlipbookComponent.PlayFromStart` _loading)
      (`PaperFlipbookComponent.SetLooping` _loading false))))

(fn `UserConstructionScript`)