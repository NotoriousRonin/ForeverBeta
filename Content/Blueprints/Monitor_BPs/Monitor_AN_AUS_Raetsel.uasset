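; Monitor puzzle where the player earns bugs by setting five monitors to the correct on/off combination (2, 4, 5 on; 1, 3 off).
; Box hits toggle monitors 1–4 between off and loading visuals, while monitor 5 only switches on and replays a second animation on further hits.
; Each state change checks the combination; winning locks input and shows win text.
; BP_Character's RaetselGeloest flag selects the larger first-solve or smaller repeat reward and sound.
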(event `testObGewonnen`
  ;[1 1 1] Testet ob Monitore in richtiger Kombination aktivirert sind
  ;;[1 0.2683 0.1826] Bedigung um Rätsel zu lösen
  (if (and (`self.isTouched_Monitor4`) (`self.isTouched_Monitor2`) (`self.isTouched_Monitor5`) (and (== (`self.isTouched_Monitor1`) false) (== (`self.isTouched_Monitor3`) false)))
    (set `self.isWon` (+ (`self.isWon`) 1))
    (if (== (`self.isWon`) 1)
      (bind _asbp_character (cast `/Game/Blueprints/BP_Character` (`GameplayStatics.GetPlayerCharacter` 0)))
      (if (`/Game/Blueprints/BP_Character.raetselGeloest` _asbp_character)
        ;;[1 1 1] Wiederholtes Lösen des Rätsel/ 5Bugs Belohnung
        (`SceneComponent.SetVisibility` (`self.Aus5`) false false)
        (`SceneComponent.SetVisibility` (`self.Loading5`) false false)
        (`SceneComponent.SetVisibility` (`self.Loading5.2`) false false)
        (`SceneComponent.SetVisibility` (`self.wonText_2`) true false)
        (bind _asbp_character_2 (cast `/Game/Blueprints/BP_Character` (`GameplayStatics.GetPlayerCharacter` 0)))
        (set `/Game/Blueprints/BP_Character.raetselGeloest` true _asbp_character_2)
        (`/Game/Blueprints/BP_Character.collectBugs` _asbp_character_2 5)
        (`GameplayStatics.SpawnSoundAtLocation` "/Game/Sound/SoundCues/Raetsel/5Items.5Items")
        (else
          ;;[1 1 1] Erstmaliges Lösen / 50 Bugs Belohnung
          (`SceneComponent.SetVisibility` (`self.Aus5`) false false)
          (`SceneComponent.SetVisibility` (`self.Loading5`) false false)
          (`SceneComponent.SetVisibility` (`self.Loading5.2`) false false)
          (`SceneComponent.SetVisibility` (`self.wonText_1`) true false)
          (bind _asbp_character_3 (cast `/Game/Blueprints/BP_Character` (`GameplayStatics.GetPlayerCharacter` 0)))
          (set `/Game/Blueprints/BP_Character.raetselGeloest` true _asbp_character_3)
          (`/Game/Blueprints/BP_Character.collectBugs` _asbp_character_3 50)
          (`GameplayStatics.SpawnSoundAtLocation` "/Game/Sound/SoundCues/Raetsel/50Items.50Items"))))))

(event `self.BoxB1.OnComponentHit`
  (params (HitComponent :type "PrimitiveComponent Object Reference") (OtherActor :type "Actor Object Reference") (OtherComp :type "PrimitiveComponent Object Reference") (NormalImpulse :type "Vector Structure") (Hit :type "HitResult Structure (by ref)"))
  (bind _aus (`self.Aus`))
  (bind _loading (`self.Loading`))
  ;[0.1904 0.9103 1] Verhalten der Monitore
  (if (== (`self.isWon`) 0)
    (if (`self.isTouched_Monitor1`)
      (set `self.isTouched_Monitor1` false)
      (`KismetSystemLibrary.PrintString` "AUS")
      (`SceneComponent.SetVisibility` _aus true false)
      (`SceneComponent.SetVisibility` _loading false false)
      (else
        (set `self.isTouched_Monitor1` true)
        (`KismetSystemLibrary.PrintString` "AN")
        (`SceneComponent.SetVisibility` _aus false false)
        (`SceneComponent.SetVisibility` _loading true false)
        (`PaperFlipbookComponent.PlayFromStart` _loading)
        (`PaperFlipbookComponent.SetLooping` _loading false)))
    (`self.testObGewonnen`)))

(event `self.BoxB2.OnComponentHit`
  (params (HitComponent :type "PrimitiveComponent Object Reference") (OtherActor :type "Actor Object Reference") (OtherComp :type "PrimitiveComponent Object Reference") (NormalImpulse :type "Vector Structure") (Hit :type "HitResult Structure (by ref)"))
  (bind _aus2 (`self.Aus2`))
  (bind _loading2 (`self.Loading2`))
  ;[0.1904 0.9103 1] Verhalten der Monitore
  (if (== (`self.isWon`) 0)
    (if (`self.isTouched_Monitor2`)
      (set `self.isTouched_Monitor2` false)
      (`KismetSystemLibrary.PrintString` "AUS")
      (`SceneComponent.SetVisibility` _aus2 true false)
      (`SceneComponent.SetVisibility` _loading2 false false)
      (else
        (set `self.isTouched_Monitor2` true)
        (`KismetSystemLibrary.PrintString` "AN")
        (`SceneComponent.SetVisibility` _aus2 false false)
        (`SceneComponent.SetVisibility` _loading2 true false)
        (`PaperFlipbookComponent.PlayFromStart` _loading2)
        (`PaperFlipbookComponent.SetLooping` _loading2 false)))
    (`self.testObGewonnen`)))

(event `self.BoxB3.OnComponentHit`
  (params (HitComponent :type "PrimitiveComponent Object Reference") (OtherActor :type "Actor Object Reference") (OtherComp :type "PrimitiveComponent Object Reference") (NormalImpulse :type "Vector Structure") (Hit :type "HitResult Structure (by ref)"))
  (bind _aus3 (`self.Aus3`))
  (bind _loading3 (`self.Loading3`))
  ;[0.1904 0.9103 1] Verhalten der Monitore
  (if (== (`self.isWon`) 0)
    (if (`self.isTouched_Monitor3`)
      (set `self.isTouched_Monitor3` false)
      (`KismetSystemLibrary.PrintString` "AUS")
      (`SceneComponent.SetVisibility` _aus3 true false)
      (`SceneComponent.SetVisibility` _loading3 false false)
      (else
        (set `self.isTouched_Monitor3` true)
        (`KismetSystemLibrary.PrintString` "AN")
        (`SceneComponent.SetVisibility` _aus3 false false)
        (`SceneComponent.SetVisibility` _loading3 true false)
        (`PaperFlipbookComponent.PlayFromStart` _loading3)
        (`PaperFlipbookComponent.SetLooping` _loading3 false)))
    (`self.testObGewonnen`)))

(event `self.BoxB4.OnComponentHit`
  (params (HitComponent :type "PrimitiveComponent Object Reference") (OtherActor :type "Actor Object Reference") (OtherComp :type "PrimitiveComponent Object Reference") (NormalImpulse :type "Vector Structure") (Hit :type "HitResult Structure (by ref)"))
  (bind _aus4 (`self.Aus4`))
  (bind _loading4 (`self.Loading4`))
  ;[0.1904 0.9103 1] Verhalten der Monitore
  (if (== (`self.isWon`) 0)
    (if (`self.isTouched_Monitor4`)
      (set `self.isTouched_Monitor4` false)
      (`KismetSystemLibrary.PrintString` "AUS")
      (`SceneComponent.SetVisibility` _aus4 true false)
      (`SceneComponent.SetVisibility` _loading4 false false)
      (else
        (set `self.isTouched_Monitor4` true)
        (`KismetSystemLibrary.PrintString` "AN")
        (`SceneComponent.SetVisibility` _aus4 false false)
        (`SceneComponent.SetVisibility` _loading4 true false)
        (`PaperFlipbookComponent.PlayFromStart` _loading4)
        (`PaperFlipbookComponent.SetLooping` _loading4 false)))
    (`self.testObGewonnen`)))

(event `self.BoxA5.OnComponentHit`
  (params (HitComponent :type "PrimitiveComponent Object Reference") (OtherActor :type "Actor Object Reference") (OtherComp :type "PrimitiveComponent Object Reference") (NormalImpulse :type "Vector Structure") (Hit :type "HitResult Structure (by ref)"))
  (bind _loading5 (`self.Loading5`))
  (bind _loading5_2 (`self.Loading5.2`))
  ;[0.1904 0.9103 1] Verhalten der Monitore
  ;;[1 1 1] Hinweismonitor
  (if (== (`self.isWon`) 0)
    (if (`self.isTouched_Monitor5`)
      (`SceneComponent.SetVisibility` _loading5_2 true false)
      (`PaperFlipbookComponent.SetLooping` _loading5_2 false)
      (`PaperFlipbookComponent.PlayFromStart` _loading5_2)
      (else
        (set `self.isTouched_Monitor5` true)
        (`KismetSystemLibrary.PrintString` "AN")
        (`SceneComponent.SetVisibility` (`self.Aus5`) false false)
        (`SceneComponent.SetVisibility` _loading5 true false)
        (`PaperFlipbookComponent.PlayFromStart` _loading5)
        (`PaperFlipbookComponent.SetLooping` _loading5 false)
        (`self.testObGewonnen`)))))

(fn `UserConstructionScript`)