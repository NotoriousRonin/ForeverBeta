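; SpeicherKlasse, in the game's save folder, holds a top-three highscore board of player names and scores counted in bugs.
; setHighscore puts the new name and score in first place and shifts the older entries down, dropping the third, without comparing scores.
; Three getter functions format each place as a display string of player name, score and a "Bugs" suffix.
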(event `setHighscore`
  (params (NewParam :type Text) (NewParam2 :type Integer))
  (`|ExecutionSequence`
    (:`then_0`
      (set `self.3_Highscore` (`self.2_Highscore`))
      (set `self.2_Highscore` (`self.1_Highscore`))
      (set `self.1_Highscore` NewParam2))
    (:`then_1`
      (set `self.3_Player` (`self.2_Player`))
      (set `self.2_Player` (`self.1_Player`))
      (set `self.1_Player` NewParam))))

(fn `GetDritterPlatzText`
  (returns (zweiterPlatzText :type String))
  (return (`KismetStringLibrary.BuildString_Int` (`KismetTextLibrary.Conv_TextToString` (`self.3_Player`)) ":     " (`self.3_Highscore`) "Bugs")))

(fn `GetErsterPlatzText`
  (params (Platzierung :type Integer))
  (returns (ErsterPlatzText :type String))
  (return (`KismetStringLibrary.BuildString_Int` (`KismetTextLibrary.Conv_TextToString` (`self.1_Player`)) ":     " (`self.1_Highscore`) "Bugs")))

(fn `GetZweiterPlatzText`
  (returns (zweiterPlatzText :type String))
  (return (`KismetStringLibrary.BuildString_Int` (`KismetTextLibrary.Conv_TextToString` (`self.2_Player`)) ":     " (`self.2_Highscore`) "Bugs")))